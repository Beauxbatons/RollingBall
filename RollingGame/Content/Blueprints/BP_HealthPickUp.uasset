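; BP_HealthPickUp is a pickup that restores health to the ball actor that collects it.
; On pickup it casts the other actor to BP_Ball, increments its health by HealthAmount, then runs the parent pickup logic, which is skipped if the cast fails.
; BeginPlay zeroes the Points value before calling the parent.
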(event `self.ReceiveBeginPlay`
  (set `self.Points` 0)
  (`parent.ReceiveBeginPlay`))

(event `self.On Pick Up`
  (params (OtherActor :type "Object Object Reference"))
  (bind _asbp_ball (cast `/Game/Blueprints/BP_Ball` OtherActor))
  (`/Game/Blueprints/BP_Ball.IncrementHealth` _asbp_ball (`self.HealthAmount`))
  (`parent.On Pick Up` OtherActor))

(fn `UserConstructionScript`
  (`parent.UserConstructionScript`))