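; BP_Button is a pressable button that triggers linked actors when a BP_Ball overlaps its sphere.
; On press it plays a sound, recolors its dynamic material and runs a timeline that shifts the button vertically.
; It then calls OnPickUp on each BP_Button or BP_EventLauncher in AffectedActors.
; Its own OnPickUp restores the unpressed state, changing the color and reversing the timeline, so buttons can reset one another.
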(event `self.ReceiveBeginPlay`
  (set `self.ButtonStartLocation` (`SceneComponent.K2_GetComponentLocation` (`self.Button`))))

(event `self.Sphere.OnComponentBeginOverlap`
  (params (OverlappedComponent :type "PrimitiveComponent Object Reference") (OtherActor :type "Actor Object Reference") (OtherComp :type "PrimitiveComponent Object Reference") (OtherBodyIndex :type Integer) (bFromSweep :type Boolean) (SweepResult :type "HitResult Structure (by ref)"))
  (cast `/Game/Blueprints/BP_Ball` OtherActor)
  (if (not (`self.IsPressed`))
    (set `self.IsPressed` true)
    (`GameplayStatics.PlaySound2D` "/Game/Retro_8Bit_Sounds/Collectables/Cues/retro_collect_pickup_item_08_Cue.retro_collect_pickup_item_08_Cue" 1.0 1.0 0.0 null null)
    (`MaterialInstanceDynamic.SetVectorParameterValue` (`self.ButtonMaterial`) "Color" (struct :`R` 1.0 :`B` 0.043376 :`A` 1.0))
    (for _array_element (`self.AffectedActors`)
      (bind _asbp_button (cast `/Game/Blueprints/BP_Button` _array_element)
        (:`then`
          (`/Game/Blueprints/I_ButtonInterface.OnPickUp` _asbp_button))
        (:`CastFailed`
          (bind _asbp_event_launcher (cast `/Game/Blueprints/BP_EventLauncher` _array_element))
          (`/Game/Blueprints/I_ButtonInterface.OnPickUp` _asbp_event_launcher))))
    (bind (_direction _buttonelevates) (`Timeline|ButtonTimeline` :!label _label)
      (:`Update`
        (`SceneComponent.K2_SetWorldLocation` (`self.Button`) (`KismetMathLibrary.MakeVector` (.x (`self.ButtonStartLocation`)) (.y (`self.ButtonStartLocation`)) (+ (.z (`self.ButtonStartLocation`)) _buttonelevates)) false false)))))

(event `/Game/Blueprints/I_ButtonInterface.OnPickUp`
  (`MaterialInstanceDynamic.SetVectorParameterValue` (`self.ButtonMaterial`) "Color" (struct :`R` 1.0 :`G` 0.323143 :`B` 0.013702 :`A` 1.0))
  (set `self.IsPressed` false)
  (goto _label :!via `Reverse`))

(fn `UserConstructionScript`
  (bind _returnvalue (`KismetMaterialLibrary.CreateDynamicMaterialInstance` "/Game/Materials/M_Button.M_Button"))
  (bind _output_get (set `self.ButtonMaterial` _returnvalue))
  (`PrimitiveComponent.SetMaterial` (`self.Button`) 0 _output_get))