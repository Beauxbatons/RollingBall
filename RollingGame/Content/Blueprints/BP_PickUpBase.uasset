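; Base pickup actor that adds its points to a BP_Ball's score when the ball overlaps its box.
; A successful pickup plays a sound and particle burst, then either destroys itself immediately or swaps its mesh for an animated W_PickUpText score widget.
; BeginPlay hides that widget and sets its score value.
; Any overlap, ball or not, also destroys the actor after a short delay.
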(event `self.ReceiveBeginPlay`
  (bind _pickuptext (`self.PickUpText`))
  (`SceneComponent.SetVisibility` _pickuptext false false)
  (bind _asw_pick_up_text (cast `/Game/Widgets/W_PickUpText` (`WidgetComponent.GetUserWidgetObject` _pickuptext)))
  (set `/Game/Widgets/W_PickUpText.ScoreValue` (`self.Points`) _asw_pick_up_text))

(event `self.Box.OnComponentBeginOverlap`
  (params (OverlappedComponent :type "PrimitiveComponent Object Reference") (OtherActor :type "Actor Object Reference") (OtherComp :type "PrimitiveComponent Object Reference") (OtherBodyIndex :type Integer) (bFromSweep :type Boolean) (SweepResult :type "HitResult Structure (by ref)"))
  (`self.On Pick Up` OtherActor)
  (`KismetSystemLibrary.Delay` 0.75)
  (`self.K2_DestroyActor`))

(fn `On Pick Up`
  (params (OtherActor :type "Object Object Reference"))
  (bind _asbp_ball (cast `/Game/Blueprints/BP_Ball` OtherActor))
  (`/Game/Blueprints/BP_Ball.IncrementScore` _asbp_ball (`self.Points`))
  (`GameplayStatics.PlaySound2D` (`self.PickUpSound`) 1.0 1.0 0.0 null null)
  (`GameplayStatics.SpawnEmitterAtLocation` (`self.PickUpParticle`) (`self.K2_GetActorLocation`))
  (if (`self.UseScoreWidget`)
    (`SceneComponent.SetVisibility` (`self.PickUpMesh`) false false)
    (`SceneComponent.SetVisibility` (`self.PickUpText`) true false)
    (bind _asw_pick_up_text (cast `/Game/Widgets/W_PickUpText` (`WidgetComponent.GetUserWidgetObject` (`self.PickUpText`))))
    (`UserWidget.PlayAnimation` _asw_pick_up_text (`/Game/Widgets/W_PickUpText.PickUpAnimation` _asw_pick_up_text) 0.0 1 "Forward" 1.0 false)
    (else
      (`self.K2_DestroyActor`))))

(fn `UserConstructionScript`)