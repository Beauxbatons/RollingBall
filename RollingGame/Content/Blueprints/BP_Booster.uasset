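; BP_Booster is a button that launches a BP_Ball when the ball hits it.
; A hit applies a velocity-change impulse to the ball along the button's up vector and plays a retro hurt sound.
; BoosterTimeline offsets the button along that vector from its BeginPlay location, with a delayed Reverse chained from the timeline's Update to retract it.
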(event `self.ReceiveBeginPlay`
  (set `self.BoosterStartLocation` (`SceneComponent.K2_GetComponentLocation` (`self.Button`))))

(event `self.Button.OnComponentHit`
  (params (HitComponent :type "PrimitiveComponent Object Reference") (OtherActor :type "Actor Object Reference") (OtherComp :type "PrimitiveComponent Object Reference") (NormalImpulse :type "Vector Structure") (Hit :type "HitResult Structure (by ref)"))
  (bind _asbp_ball (cast `/Game/Blueprints/BP_Ball` OtherActor))
  (`PrimitiveComponent.AddImpulse` (`/Game/Blueprints/BP_Ball.BallMesh` _asbp_ball) (* (`SceneComponent.GetUpVector` (`self.Button`)) 800.0) "None" true)
  (`GameplayStatics.PlaySound2D` "/Game/Retro_8Bit_Sounds/Damage_Hurt/Cues/retro_damage_hurt_ouch_01_Cue.retro_damage_hurt_ouch_01_Cue" 1.0 1.0 0.0 null null)
  (bind (_direction _boosterlaunchelevation) (`Timeline|BoosterTimeline` :!label _label)
    (:`Update`
      (`SceneComponent.K2_SetWorldLocation` (`self.Button`) (+ (`self.BoosterStartLocation`) (* (`SceneComponent.GetUpVector` (`self.Button`)) _boosterlaunchelevation)) false false)
      (`KismetSystemLibrary.Delay` 0.5)
      (goto _label :!via `Reverse`))))

(fn `UserConstructionScript`)