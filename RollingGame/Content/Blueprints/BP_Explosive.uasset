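; BP_Explosive is a hazard pickup that damages the ball player and blasts it away.
; BeginPlay configures the parent pickup with explosion effects, no score, and a looping-style spark sound stored for later shutoff.
; On pickup it decrements BP_Ball health, applies a radial impulse from below its location, then defers to the parent.
; It also binds to the ball's destroy-hazards event, which sparkles and removes it after a short delay.
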(event `self.ReceiveBeginPlay`
  (set `self.Points` 0)
  (set `self.UseScoreWidget` false)
  (set `self.PickUpSound` "/Game/StarterContent/Audio/Explosion_Cue.Explosion_Cue")
  (set `self.PickUpParticle` "/Game/StarterContent/Particles/P_Explosion.P_Explosion")
  (bind _returnvalue (`GameplayStatics.SpawnSoundAtLocation` "/Game/StarterContent/Audio/Fire_Sparks01_Cue.Fire_Sparks01_Cue" (`self.K2_GetActorLocation`) (struct) 1.0 1.0 0.0 null null))
  (set `self.SparkSound` _returnvalue)
  (`parent.ReceiveBeginPlay`)
  (add `/Game/Blueprints/BP_Ball.DestroyHazards` (cast `/Game/Blueprints/BP_Ball` (`GameplayStatics.GetPlayerPawn` 0) :!pure true) (delegate `DestroyExplosive`)))

(event `DestroyExplosive`
  (`GameplayStatics.SpawnEmitterAtLocation` "/Game/InfinityBladeEffects/Effects/FX_Treasure/Gold_Bag/P_GoldSparkle_Bag_Lo_2.P_GoldSparkle_Bag_Lo_2" (`self.K2_GetActorLocation`))
  (`KismetSystemLibrary.Delay` 0.5)
  (`ActorComponent.SetActive` (`self.SparkSound`) false false)
  (`self.K2_DestroyActor`))

(event `self.On Pick Up`
  (params (OtherActor :type "Object Object Reference"))
  (bind _asbp_ball (cast `/Game/Blueprints/BP_Ball` OtherActor))
  (`/Game/Blueprints/BP_Ball.DecrementHealth` _asbp_ball (`self.Damage`))
  (`PrimitiveComponent.AddRadialImpulse` (`/Game/Blueprints/BP_Ball.BallMesh` _asbp_ball) (`KismetMathLibrary.MakeVector` (.x (`self.K2_GetActorLocation`)) (.y (`self.K2_GetActorLocation`)) (+ (.z (`self.K2_GetActorLocation`)) -50.0)) 500.0 1000.0 "RIF_Constant" true)
  (`ActorComponent.SetActive` (`self.SparkSound`) false false)
  (`parent.On Pick Up` OtherActor))

(fn `UserConstructionScript`
  (`parent.UserConstructionScript`))